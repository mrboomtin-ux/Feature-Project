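; BP_Pawn is a player pawn that moves around and places blocks in the world.
; On BeginPlay it registers the IMC_PlayerControls Enhanced Input context on BP_PlayerController, and IA_Move drives movement along the pawn's forward and right vectors.
; Left click line-traces from the camera against world and physics objects, spawning BP_Block at the hit point.
; The hit location passes through a grid snap, but its grid size of zero leaves it unsnapped.
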(event `self.ReceiveBeginPlay`
  ; Reference to PlayerController and Mapping Context
  (bind _asbp_player_controller (cast `/Game/Blueprints/BP_PlayerController` (`GameplayStatics.GetPlayerController` 0)))
  (bind _output_get (set `self.As BP Player Controller` _asbp_player_controller))
  (bind _returnvalue (pcsubsystem `EnhancedInputLocalPlayerSubsystem` _output_get))
  (`/Engine/EditorBlueprintResources/StandardMacros.IsValid` _returnvalue
    (:`Is Valid`
      (`EnhancedInputSubsystemInterface.AddMappingContext` _returnvalue "/Game/Blueprints/InputActions/IMC_PlayerControls.IMC_PlayerControls" 0 (struct)))))

(event `EnhancedInput|/Game/Blueprints/InputActions/IA_Move`
  (params (ActionValue :type "Vector2D Structure") (ElapsedSeconds :type "Float (double-precision)") (TriggeredSeconds :type "Float (double-precision)") (InputAction :type "InputAction Object Reference" :default "/Game/Blueprints/InputActions/IA_Move.IA_Move"))
  (:`Triggered`
    (`self.AddMovementInput` (`KismetMathLibrary.GetRightVector` (struct)) ActionValue_X)
    (`self.AddMovementInput` (`self.GetActorForwardVector`) ActionValue_Y)))

(event `EnhancedInput|/Game/Blueprints/InputActions/IA_LeftClick`
  (params (ActionValue :type Boolean) (ElapsedSeconds :type "Float (double-precision)") (TriggeredSeconds :type "Float (double-precision)") (InputAction :type "InputAction Object Reference" :default "/Game/Blueprints/InputActions/IA_LeftClick.IA_LeftClick"))
  (bind _camera (`self.Camera`))
  (bind _returnvalue (`SceneComponent.K2_GetComponentLocation` _camera))
  ; Code to Place Blocks
  (:`Triggered`
    (bind (_outhit _returnvalue_2) (`KismetSystemLibrary.LineTraceSingleForObjects` _returnvalue (+ _returnvalue (* (`SceneComponent.GetForwardVector` _camera) (`self.Magnitude`))) (`|MakeArray` "ObjectTypeQuery1" "ObjectTypeQuery2" "ObjectTypeQuery4" :!type "EObjectTypeQuery Enum")))
    (if _returnvalue_2
      (`|SpawnActorFromClass` "/Game/Blueprints/BP_Block.BP_Block_C" (`KismetMathLibrary.Conv_VectorToTransform` (`KismetMathLibrary.Vector_SnappedToGrid` (`.Location` (`GameplayStatics.BreakHitResult` _outhit)))) "Undefined" "MultiplyWithRoot" null null))))

(fn `UserConstructionScript`)