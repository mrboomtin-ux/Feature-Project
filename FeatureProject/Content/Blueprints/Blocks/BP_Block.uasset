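; BP_Block is a block actor that leaves a pickup behind when it is destroyed.
; Its Destroy event calls SpawnBlock, then removes the actor.
; Despite its name, SpawnBlock spawns a single BP_Pickup at the block's location, scattered by random horizontal offsets and a slight upward one.
; The construction script and NewFunction are empty.
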(event `Destroy`
  ; Destroyed
  (`self.Spawn Block`)
  (`self.K2_DestroyActor`))

(event `Spawn Block`
  (bind _returnvalue (`KismetMathLibrary.RandomInteger64InRange` -200 200))
  (bind _returnvalue_2 (`self.GetTransform`))
  ; Spawns Block Before Destroyed
  (`|SpawnActorFromClass` "/Game/Blueprints/Blocks/Pickups/BP_Pickup.BP_Pickup_C" (`KismetMathLibrary.MakeTransform` (`KismetMathLibrary.MakeVector` (`KismetMathLibrary.Conv_Int64ToDouble` (+ (.x (.location _returnvalue_2)) _returnvalue)) (`KismetMathLibrary.Conv_Int64ToDouble` (+ (.y (.location _returnvalue_2)) _returnvalue)) (`KismetMathLibrary.Conv_Int64ToDouble` (+ (.z (.location _returnvalue_2)) (`KismetMathLibrary.RandomInteger64InRange` 0 20))))) "Undefined" "MultiplyWithRoot" null null))

(fn `NewFunction`)

(fn `UserConstructionScript`)