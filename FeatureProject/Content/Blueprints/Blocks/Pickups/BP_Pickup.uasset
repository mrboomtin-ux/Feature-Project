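; BP_Pickup is a pickup actor that bobs vertically until it is picked up.
; Tick moves it by a local offset from MoveSpeed and MoveDir, flipping the direction's Z whenever its world height passes fixed lower or upper limits.
; Those limits are absolute world Z values, so the bounce ignores where the actor is placed.
; OnPickedUp prints a debug message and destroys the actor.
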(event `/Game/Blueprints/BPI_Collectable.OnPickedUp`
  (params (`Interacting Player` :type "/Game/Blueprints/BP_Pawn Object Reference"))
  (`KismetSystemLibrary.PrintString` "Picked Up")
  (`self.K2_DestroyActor`))

(event `self.ReceiveTick`
  (params (DeltaSeconds :type "Float (single-precision)"))
  ; Bounce up and down
  (`self.K2_AddActorLocalOffset` (* DeltaSeconds (`self.Move Speed`) (`self.Move Dir`)))
  (if (<= (.z (.location (`self.GetTransform`))) -20.0)
    (set `self.Move Dir` (* (`self.Move Dir`) (0.0 0.0 -1.0)))
    (elif (>= (.z (.location (`self.GetTransform`))) 1.0)
      (set `self.Move Dir` (* (`self.Move Dir`) (0.0 0.0 -1.0))))))

(fn `UserConstructionScript`)